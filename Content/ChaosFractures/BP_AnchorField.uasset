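; BP_AnchorField is a Chaos field actor that anchors fracture pieces inside a box volume by setting their dynamic state to static.
; Its construction script builds a box falloff from the CullingArea transform and uses it to cull a uniform static-state integer outside that box.
; The result feeds a dynamic-state field command on the FieldSystemComponent.
; BeginPlay only adds an empty command with no physics type, alongside some unused nodes.
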(event `self.ReceiveBeginPlay`
  (`FieldSystemComponent.AddFieldCommand` (`self.FieldSystemComponent`) true "Field_None" null null))

(fn `UserConstructionScript`
  (`FieldSystemComponent.AddFieldCommand` (`self.FieldSystemComponent`) true "Field_DynamicState" null (`CullingField.SetCullingField` (`self.CullingField`) (`BoxFalloff.SetBoxFalloff` (`self.BoxFalloff`) 1.0 0.0 1.0 0.0 (`SceneComponent.K2_GetComponentToWorld` (`self.CullingArea`)) "Field_FallOff_None") (`UniformInteger.SetUniformInteger` (`self.UniformInteger`) (`KismetMathLibrary.Conv_ByteToInt` (`self.Static State`))) "Field_Culling_Outside")))